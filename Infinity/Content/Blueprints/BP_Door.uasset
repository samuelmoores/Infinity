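; BP_Door is a sliding door that opens when its Open event is called and closes once the player walks away.
; Open and Close each play their own timeline, lerping the mesh's relative X position between the closed and slid-aside positions and updating IsOpen.
; BeginPlay caches the player character, and ActorEndOverlap calls Close when that player leaves while the door is open.
; Nothing in this Blueprint calls Open, so the trigger comes from outside.
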(event `self.ReceiveBeginPlay`
  (bind _asbp_player_character (cast `/Game/Blueprints/BP_PlayerCharacter` (`GameplayStatics.GetPlayerCharacter` 0)))
  (set `self.PlayerCharacter` _asbp_player_character))

(event `Open`
  (bind (_direction _newtrack_0) (`Timeline|OpenTimeline` :!via `PlayFromStart`)
    (:`Update`
      (`SceneComponent.K2_SetRelativeLocation` (`self.Mesh`) (`KismetMathLibrary.VLerp` (0.0 0.0 0.0) (-315.0 0.0 0.0) _newtrack_0) false false)
      (set `self.isOpen` true))))

(event `self.ReceiveActorEndOverlap`
  (params (OtherActor :type "Actor Object Reference"))
  (if (and (== OtherActor (`self.PlayerCharacter`)) (`self.isOpen`))
    (`self.Close`)))

(event `Close`
  (bind (_direction _newtrack_0) (`Timeline|Timeline` :!via `PlayFromStart`)
    (:`Update`
      (`SceneComponent.K2_SetRelativeLocation` (`self.Mesh`) (`KismetMathLibrary.VLerp` (-315.0 0.0 0.0) (0.0 0.0 0.0) _newtrack_0) false false)
      (set `self.isOpen` false))))

(fn `UserConstructionScript`)