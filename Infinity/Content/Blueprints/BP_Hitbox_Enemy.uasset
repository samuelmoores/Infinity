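; Enemy hitbox Blueprint that positions a HitBox component and styles it by hitbox type.
; DisplayHitbox switches on the type to apply the proximity or strike material, while the Hurt Box case targets material slot 2 with no material assigned.
; It then moves the component to HitboxLocation and sets it invisible, despite the function's name.
; The event graph and construction script are empty, and no overlap or damage logic exists here.
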(fn `DisplayHitbox`
  (params (HitboxType :type "EHitboxEnum Enum" :default "HB_PROXIMITY"))
  (switch `EHitboxEnum` HitboxType
    (:`HB_PROXIMITY`
      (`PrimitiveComponent.SetMaterial` (`self.HitBox`) 0 "/Game/Environment/Materials/HitBoxMaterials/M_ProximityHitbox.M_ProximityHitbox"))
    (:`HB_STRIKE`
      (`PrimitiveComponent.SetMaterial` (`self.HitBox`) 0 "/Game/Environment/Materials/HitBoxMaterials/M_StrikeHitbox.M_StrikeHitbox"))
    (:`HB_HURTBOX`
      (`PrimitiveComponent.SetMaterial` (`self.HitBox`) 2 null)))
  (`SceneComponent.K2_SetWorldLocation` (`self.HitBox`) (`self.HitboxLocation`) false false)
  (`SceneComponent.SetVisibility` (`self.HitBox`) false false))

(fn `UserConstructionScript`)