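; BP_HitboxEnemy is an enemy attack hitbox actor that tracks whether an attack would hit the player.
; MissedAttack starts true, turns false when an actor tagged Player begins overlapping and returns to true when it leaves.
; DisplayHitbox shows the HitboxEnemy component by applying the proximity hitbox material, moving it to HitboxLocation and making it visible.
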(event `self.ReceiveBeginPlay`
  (set `self.missedAttack` true))

(event `self.ReceiveTick`
  (params (DeltaSeconds :type "Float (single-precision)")))

(event `self.ReceiveActorBeginOverlap`
  (params (OtherActor :type "Actor Object Reference"))
  (if (`self.ActorHasTag` OtherActor "Player")
    (set `self.missedAttack` false)))

(event `self.ReceiveActorEndOverlap`
  (params (OtherActor :type "Actor Object Reference"))
  (if (`self.ActorHasTag` OtherActor "Player")
    (set `self.missedAttack` true)))

(fn `Display Hitbox`
  (`PrimitiveComponent.SetMaterial` (`self.HitboxEnemy`) 0 "/Game/Environment/Materials/HitBoxMaterials/M_ProximityHitbox.M_ProximityHitbox")
  (`SceneComponent.K2_SetWorldLocation` (`self.HitboxEnemy`) (`self.HitboxLocation`) false false)
  (`SceneComponent.SetVisibility` (`self.HitboxEnemy`) true false))

(fn `UserConstructionScript`)