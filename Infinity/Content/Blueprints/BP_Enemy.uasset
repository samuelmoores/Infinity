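; BP_Enemy is an enemy Blueprint that displays its health on a HealthBar widget component.
; BeginPlay caches the player character and the bar's WBP_EnemyHealth widget.
; Each Tick, UpdateHealthBar billboards the bar by copying the follow camera's rotation with yaw turned 180 degrees, then pushes Health into the widget.
; The widget is hidden when Dead is set; this graph only reads Health and Dead.
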(event `self.ReceiveBeginPlay`
  (bind _asbp_third_person_character (cast `/Game/ThirdPerson/Blueprints/BP_ThirdPersonCharacter` (`GameplayStatics.GetPlayerCharacter` 0)))
  (set `self.Player` _asbp_third_person_character)
  (bind _aswbp_enemy_health (cast `/Game/UI/WBP_EnemyHealth` (`WidgetComponent.GetUserWidgetObject` (`self.HealthBar`))))
  (set `self.EnemyHealthWidget` _aswbp_enemy_health))

(event `self.ReceiveTick`
  (params (DeltaSeconds :type "Float (single-precision)"))
  (`/Engine/EditorBlueprintResources/StandardMacros.IsValid` (`self.Player`)
    (:`Is Valid`
      (`self.UpdateHealthBar`))))

(fn `UpdateHealthBar`
  (bind _followcamera (`InfinityCharacter.FollowCamera` (`self.Player`)))
  (bind (_returnvalue_roll _returnvalue_pitch _returnvalue_yaw) (`KismetMathLibrary.BreakRotator` (`SceneComponent.K2_GetComponentRotation` _followcamera)))
  (`/Engine/EditorBlueprintResources/StandardMacros.IsValid` _followcamera
    (:`Is Valid`
      (`SceneComponent.K2_SetWorldRotation` (`self.HealthBar`) (`KismetMathLibrary.MakeRotator` _returnvalue_roll _returnvalue_pitch (+ _returnvalue_yaw 180.0)) false false)
      (set `/Game/UI/WBP_EnemyHealth.Health` (`self.health`) (`self.EnemyHealthWidget`))
      (if (`self.dead`)
        (`Widget.SetVisibility` (`self.EnemyHealthWidget`) "Hidden")))))

(fn `UserConstructionScript`)